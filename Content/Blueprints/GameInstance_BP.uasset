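; Game instance Blueprint that hosts and joins LAN multiplayer sessions.
; HostGame creates a four-connection session, sets the Stage enum and opens Scene_01 as a listen server.
; JoinGame searches for LAN sessions, joins the first result without checking for an empty list, and sets the same Stage on success.
; Session failures only print a message.
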(event `Host Game`
  (params (playerController :type "/Game/Blueprints/PlayerController_BP Object Reference"))
  ;[1 1 1] Host Game
  (`CreateSessionCallbackProxy.CreateSession` playerController 4 true
    (:`OnSuccess`
      (set `self.Stage` "NewEnumerator1")
      (`GameplayStatics.OpenLevel` "Scene_01" true "listen"))
    (:`OnFailure`
      (`KismetSystemLibrary.PrintString` "Failure creating session"))))

(event `Join Game`
  (params (playerController :type "/Game/Blueprints/PlayerController_BP Object Reference"))
  ;[1 1 1] Join Game
  (bind _results (`FindSessionsCallbackProxy.FindSessions` playerController 20 true)
    (:`OnSuccess`
      (`JoinSessionCallbackProxy.JoinSession` playerController (`|GetArrayItem` _results)
        (:`OnSuccess`
          (set `self.Stage` "NewEnumerator1"))
        (:`OnFailure`
          (`KismetSystemLibrary.PrintString` "Failure joining session"))))
    (:`OnFailure`
      (`KismetSystemLibrary.PrintString` "Game session not found" true true (struct :`G` 0.66 :`B` 1.0 :`A` 1.0) 5.0))))