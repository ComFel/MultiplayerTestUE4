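; Player controller that creates the menu widget matching the game stage and handles the pause menu input.
; On BeginPlay it reads Stage from GameInstance_BP and, for the local controller only, shows MainMenu with the cursor during Login or InGameMenu_01 without it during Playing.
; The Show Pause Menu input forwards to the stored in-game widget, which is only assigned in the Playing stage.
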(event `self.ReceiveBeginPlay`
  (bind _returnvalue (`self.IsLocalPlayerController`))
  ;[1 1 1] Se establece la etapa del juego
  (bind _asgame_instance_bp (cast `/Game/Blueprints/GameInstance_BP` (`GameplayStatics.GetGameInstance`)))
  (switch `/Game/Blueprints/GameStage` (`/Game/Blueprints/GameInstance_BP.Stage` _asgame_instance_bp)
    (:`NewEnumerator0`
      (if _returnvalue
        ;[1 1 1] Main Menú
        (bind _returnvalue_2 (`|CreateWidget` "/Game/Blueprints/MainMenu.MainMenu_C" self))
        (`UserWidget.AddToViewport` _returnvalue_2 0)
        (set `self.bShowMouseCursor` true)))
    (:`NewEnumerator1`
      (if _returnvalue
        ;[1 1 1] In-game Menú
        (bind _returnvalue_3 (`|CreateWidget` "/Game/Blueprints/InGameMenu_01.InGameMenu_01_C" self))
        (bind _output_get (set `self.InGameWidget` _returnvalue_3))
        (`UserWidget.AddToViewport` _output_get 0)
        (set `self.bShowMouseCursor` false)))))

(event `InputAction|Show Pause Menu`
  (params (Key :type "Key Structure"))
  ;[1 1 1] Pause Menú
  (:`Pressed`
    (`/Game/Blueprints/InGameMenu_01.Show Pause Menu` (`self.InGameWidget`))))

(fn `UserConstructionScript`)