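; MyGameInstanceBP is a game instance Blueprint that handles hosting and joining two-player LAN sessions.
; HostGame creates a session for the given player controller, then sets the Stage enum and opens FirstPersonExampleMap on success.
; JoinGame searches LAN sessions and joins the first result without checking that one exists, setting the same Stage value on success.
; Failures in creating, finding or joining only print a message.
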(event `Host Game`
  (params (PlayerController :type "/Game/FirstPersonBP/Blueprints/MyPlayerController Object Reference"))
  (`CreateSessionCallbackProxy.CreateSession` PlayerController 2 true
    (:`OnSuccess`
      (set `self.Stage` "NewEnumerator1")
      (`GameplayStatics.OpenLevel` "FirstPersonExampleMap"))
    (:`OnFailure`
      (`KismetSystemLibrary.PrintString` "Fail to create session"))))

(event `Join Game`
  (params (`Player Controller` :type "/Game/FirstPersonBP/Blueprints/MyPlayerController Object Reference"))
  (bind _results (`FindSessionsCallbackProxy.FindSessions` `Player Controller` 20 true)
    (:`then`
      (`JoinSessionCallbackProxy.JoinSession` `Player Controller` (`|GetArrayItem` _results)
        (:`OnSuccess`
          (set `self.Stage` "NewEnumerator1"))
        (:`OnFailure`
          (`KismetSystemLibrary.PrintString` "Fail to join lobby"))))
    (:`OnFailure`
      (`KismetSystemLibrary.PrintString` "Not game Found"))))